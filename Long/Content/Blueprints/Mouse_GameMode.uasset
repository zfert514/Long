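; Game mode that provides camera zoom-in and zoom-out functions for a cast of named characters, one pair per person.
; Each function sets player 0's view target to the Camera, then creates a new level sequence player for that person's Move sequence.
; Zoom-in plays the sequence forward and zoom-out plays the same sequence in reverse.
; The event graph is empty, so these functions are triggered from elsewhere.
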(fn `UserConstructionScript`)

(fn `ZoomInAlyssa`
  (`PlayerController.SetViewTargetWithBlend` (`GameplayStatics.GetPlayerController` 0) (`self.Camera`) 0.0 "VTBlend_Linear" 0.0 false)
  (bind _outactor (`LevelSequencePlayer.CreateLevelSequencePlayer` "/Game/Sequences/MoveAlyssa.MoveAlyssa"))
  (`MovieSceneSequencePlayer.Play` (`LevelSequenceActor.SequencePlayer` _outactor)))

(fn `ZoomInAna`
  (`PlayerController.SetViewTargetWithBlend` (`GameplayStatics.GetPlayerController` 0) (`self.Camera`) 0.0 "VTBlend_Linear" 0.0 false)
  (bind _outactor (`LevelSequencePlayer.CreateLevelSequencePlayer` "/Game/Sequences/MoveAna.MoveAna"))
  (`MovieSceneSequencePlayer.Play` (`LevelSequenceActor.SequencePlayer` _outactor)))

(fn `ZoomInChristy`
  (`PlayerController.SetViewTargetWithBlend` (`GameplayStatics.GetPlayerController` 0) (`self.Camera`) 0.0 "VTBlend_Linear" 0.0 false)
  (bind _outactor (`LevelSequencePlayer.CreateLevelSequencePlayer` "/Game/Sequences/MoveChristy.MoveChristy"))
  (`MovieSceneSequencePlayer.Play` (`LevelSequenceActor.SequencePlayer` _outactor)))

(fn `ZoomInDani`
  (`PlayerController.SetViewTargetWithBlend` (`GameplayStatics.GetPlayerController` 0) (`self.Camera`) 0.0 "VTBlend_Linear" 0.0 false)
  (bind _outactor (`LevelSequencePlayer.CreateLevelSequencePlayer` "/Game/Sequences/MoveDani.MoveDani"))
  (`MovieSceneSequencePlayer.Play` (`LevelSequenceActor.SequencePlayer` _outactor)))

(fn `ZoomInDiamond`
  (`PlayerController.SetViewTargetWithBlend` (`GameplayStatics.GetPlayerController` 0) (`self.Camera`) 0.0 "VTBlend_Linear" 0.0 false)
  (bind _outactor (`LevelSequencePlayer.CreateLevelSequencePlayer` "/Game/Sequences/MoveDiamond.MoveDiamond"))
  (`MovieSceneSequencePlayer.Play` (`LevelSequenceActor.SequencePlayer` _outactor)))

(fn `ZoomInDoo`
  (`PlayerController.SetViewTargetWithBlend` (`GameplayStatics.GetPlayerController` 0) (`self.Camera`) 0.0 "VTBlend_Linear" 0.0 false)
  (bind _outactor (`LevelSequencePlayer.CreateLevelSequencePlayer` "/Game/Sequences/MoveDoo.MoveDoo"))
  (`MovieSceneSequencePlayer.Play` (`LevelSequenceActor.SequencePlayer` _outactor)))

(fn `ZoomInEmma`
  (`PlayerController.SetViewTargetWithBlend` (`GameplayStatics.GetPlayerController` 0) (`self.Camera`) 0.0 "VTBlend_Linear" 0.0 false)
  (bind _outactor (`LevelSequencePlayer.CreateLevelSequencePlayer` "/Game/Sequences/MoveEmm.MoveEmm"))
  (`MovieSceneSequencePlayer.Play` (`LevelSequenceActor.SequencePlayer` _outactor)))

(fn `ZoomInIvana`
  (`PlayerController.SetViewTargetWithBlend` (`GameplayStatics.GetPlayerController` 0) (`self.Camera`) 0.0 "VTBlend_Linear" 0.0 false)
  (bind _outactor (`LevelSequencePlayer.CreateLevelSequencePlayer` "/Game/Sequences/MoveIvana.MoveIvana"))
  (`MovieSceneSequencePlayer.Play` (`LevelSequenceActor.SequencePlayer` _outactor)))

(fn `ZoomInJulia`
  (`PlayerController.SetViewTargetWithBlend` (`GameplayStatics.GetPlayerController` 0) (`self.Camera`) 0.0 "VTBlend_Linear" 0.0 false)
  (bind _outactor (`LevelSequencePlayer.CreateLevelSequencePlayer` "/Game/Sequences/MoveJulia.MoveJulia"))
  (`MovieSceneSequencePlayer.Play` (`LevelSequenceActor.SequencePlayer` _outactor)))

(fn `ZoomInKerrie`
  (`PlayerController.SetViewTargetWithBlend` (`GameplayStatics.GetPlayerController` 0) (`self.Camera`) 0.0 "VTBlend_Linear" 0.0 false)
  (bind _outactor (`LevelSequencePlayer.CreateLevelSequencePlayer` "/Game/Sequences/MoveKerrie.MoveKerrie"))
  (`MovieSceneSequencePlayer.Play` (`LevelSequenceActor.SequencePlayer` _outactor)))

(fn `ZoomInSavannah`
  (`PlayerController.SetViewTargetWithBlend` (`GameplayStatics.GetPlayerController` 0) (`self.Camera`) 0.0 "VTBlend_Linear" 0.0 false)
  (bind _outactor (`LevelSequencePlayer.CreateLevelSequencePlayer` "/Game/Sequences/MoveSavannah.MoveSavannah"))
  (`MovieSceneSequencePlayer.Play` (`LevelSequenceActor.SequencePlayer` _outactor)))

(fn `ZoomInSophia`
  (`PlayerController.SetViewTargetWithBlend` (`GameplayStatics.GetPlayerController` 0) (`self.Camera`) 0.0 "VTBlend_Linear" 0.0 false)
  (bind _outactor (`LevelSequencePlayer.CreateLevelSequencePlayer` "/Game/Sequences/MoveSophia.MoveSophia"))
  (`MovieSceneSequencePlayer.Play` (`LevelSequenceActor.SequencePlayer` _outactor)))

(fn `ZoomInTy`
  (`PlayerController.SetViewTargetWithBlend` (`GameplayStatics.GetPlayerController` 0) (`self.Camera`) 0.0 "VTBlend_Linear" 0.0 false)
  (bind _outactor (`LevelSequencePlayer.CreateLevelSequencePlayer` "/Game/Sequences/MoveTyrell.MoveTyrell"))
  (`MovieSceneSequencePlayer.Play` (`LevelSequenceActor.SequencePlayer` _outactor)))

(fn `ZoomInZack`
  (`PlayerController.SetViewTargetWithBlend` (`GameplayStatics.GetPlayerController` 0) (`self.Camera`) 0.0 "VTBlend_Linear" 0.0 false)
  (bind _outactor (`LevelSequencePlayer.CreateLevelSequencePlayer` "/Game/Sequences/MoveZack.MoveZack"))
  (`MovieSceneSequencePlayer.Play` (`LevelSequenceActor.SequencePlayer` _outactor)))

(fn `ZoomOutAlyssa`
  (`PlayerController.SetViewTargetWithBlend` (`GameplayStatics.GetPlayerController` 0) (`self.Camera`) 0.0 "VTBlend_Linear" 0.0 false)
  (bind _outactor (`LevelSequencePlayer.CreateLevelSequencePlayer` "/Game/Sequences/MoveAlyssa.MoveAlyssa"))
  (`MovieSceneSequencePlayer.PlayReverse` (`LevelSequenceActor.SequencePlayer` _outactor)))

(fn `ZoomOutAna`
  (`PlayerController.SetViewTargetWithBlend` (`GameplayStatics.GetPlayerController` 0) (`self.Camera`) 0.0 "VTBlend_Linear" 0.0 false)
  (bind _outactor (`LevelSequencePlayer.CreateLevelSequencePlayer` "/Game/Sequences/MoveAna.MoveAna"))
  (`MovieSceneSequencePlayer.PlayReverse` (`LevelSequenceActor.SequencePlayer` _outactor)))

(fn `ZoomOutChristy`
  (`PlayerController.SetViewTargetWithBlend` (`GameplayStatics.GetPlayerController` 0) (`self.Camera`) 0.0 "VTBlend_Linear" 0.0 false)
  (bind _outactor (`LevelSequencePlayer.CreateLevelSequencePlayer` "/Game/Sequences/MoveChristy.MoveChristy"))
  (`MovieSceneSequencePlayer.PlayReverse` (`LevelSequenceActor.SequencePlayer` _outactor)))

(fn `ZoomOutDani`
  (`PlayerController.SetViewTargetWithBlend` (`GameplayStatics.GetPlayerController` 0) (`self.Camera`) 0.0 "VTBlend_Linear" 0.0 false)
  (bind _outactor (`LevelSequencePlayer.CreateLevelSequencePlayer` "/Game/Sequences/MoveDani.MoveDani"))
  (`MovieSceneSequencePlayer.PlayReverse` (`LevelSequenceActor.SequencePlayer` _outactor)))

(fn `ZoomOutDiamond`
  (`PlayerController.SetViewTargetWithBlend` (`GameplayStatics.GetPlayerController` 0) (`self.Camera`) 0.0 "VTBlend_Linear" 0.0 false)
  (bind _outactor (`LevelSequencePlayer.CreateLevelSequencePlayer` "/Game/Sequences/MoveDiamond.MoveDiamond"))
  (`MovieSceneSequencePlayer.PlayReverse` (`LevelSequenceActor.SequencePlayer` _outactor)))

(fn `ZoomOutDoo`
  (`PlayerController.SetViewTargetWithBlend` (`GameplayStatics.GetPlayerController` 0) (`self.Camera`) 0.0 "VTBlend_Linear" 0.0 false)
  (bind _outactor (`LevelSequencePlayer.CreateLevelSequencePlayer` "/Game/Sequences/MoveDoo.MoveDoo"))
  (`MovieSceneSequencePlayer.PlayReverse` (`LevelSequenceActor.SequencePlayer` _outactor)))

(fn `ZoomOutEmma`
  (`PlayerController.SetViewTargetWithBlend` (`GameplayStatics.GetPlayerController` 0) (`self.Camera`) 0.0 "VTBlend_Linear" 0.0 false)
  (bind _outactor (`LevelSequencePlayer.CreateLevelSequencePlayer` "/Game/Sequences/MoveEmm.MoveEmm"))
  (`MovieSceneSequencePlayer.PlayReverse` (`LevelSequenceActor.SequencePlayer` _outactor)))

(fn `ZoomOutIvana`
  (`PlayerController.SetViewTargetWithBlend` (`GameplayStatics.GetPlayerController` 0) (`self.Camera`) 0.0 "VTBlend_Linear" 0.0 false)
  (bind _outactor (`LevelSequencePlayer.CreateLevelSequencePlayer` "/Game/Sequences/MoveIvana.MoveIvana"))
  (`MovieSceneSequencePlayer.PlayReverse` (`LevelSequenceActor.SequencePlayer` _outactor)))

(fn `ZoomOutJulia`
  (`PlayerController.SetViewTargetWithBlend` (`GameplayStatics.GetPlayerController` 0) (`self.Camera`) 0.0 "VTBlend_Linear" 0.0 false)
  (bind _outactor (`LevelSequencePlayer.CreateLevelSequencePlayer` "/Game/Sequences/MoveJulia.MoveJulia"))
  (`MovieSceneSequencePlayer.PlayReverse` (`LevelSequenceActor.SequencePlayer` _outactor)))

(fn `ZoomOutKerrie`
  (`PlayerController.SetViewTargetWithBlend` (`GameplayStatics.GetPlayerController` 0) (`self.Camera`) 0.0 "VTBlend_Linear" 0.0 false)
  (bind _outactor (`LevelSequencePlayer.CreateLevelSequencePlayer` "/Game/Sequences/MoveKerrie.MoveKerrie"))
  (`MovieSceneSequencePlayer.PlayReverse` (`LevelSequenceActor.SequencePlayer` _outactor)))

(fn `ZoomOutSavannah`
  (`PlayerController.SetViewTargetWithBlend` (`GameplayStatics.GetPlayerController` 0) (`self.Camera`) 0.0 "VTBlend_Linear" 0.0 false)
  (bind _outactor (`LevelSequencePlayer.CreateLevelSequencePlayer` "/Game/Sequences/MoveSavannah.MoveSavannah"))
  (`MovieSceneSequencePlayer.PlayReverse` (`LevelSequenceActor.SequencePlayer` _outactor)))

(fn `ZoomOutSophia`
  (`PlayerController.SetViewTargetWithBlend` (`GameplayStatics.GetPlayerController` 0) (`self.Camera`) 0.0 "VTBlend_Linear" 0.0 false)
  (bind _outactor (`LevelSequencePlayer.CreateLevelSequencePlayer` "/Game/Sequences/MoveSophia.MoveSophia"))
  (`MovieSceneSequencePlayer.PlayReverse` (`LevelSequenceActor.SequencePlayer` _outactor)))

(fn `ZoomOutTy`
  (`PlayerController.SetViewTargetWithBlend` (`GameplayStatics.GetPlayerController` 0) (`self.Camera`) 0.0 "VTBlend_Linear" 0.0 false)
  (bind _outactor (`LevelSequencePlayer.CreateLevelSequencePlayer` "/Game/Sequences/MoveTyrell.MoveTyrell"))
  (`MovieSceneSequencePlayer.PlayReverse` (`LevelSequenceActor.SequencePlayer` _outactor)))

(fn `ZoomOutZack`
  (`PlayerController.SetViewTargetWithBlend` (`GameplayStatics.GetPlayerController` 0) (`self.Camera`) 0.0 "VTBlend_Linear" 0.0 false)
  (bind _outactor (`LevelSequencePlayer.CreateLevelSequencePlayer` "/Game/Sequences/MoveZack.MoveZack"))
  (`MovieSceneSequencePlayer.PlayReverse` (`LevelSequenceActor.SequencePlayer` _outactor)))